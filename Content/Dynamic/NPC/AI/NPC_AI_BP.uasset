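; AI controller for a guard NPC that starts the GuardBehavior tree with the PatrolData blackboard on BeginPlay.
; On perception updates, it checks the last sight and hearing stimuli of any actor not tagged Enemy.
; Successful senses set SeesPlayer or HearsPlayer, LastKnownLocation and the Enemy target; failed ones reset that flag and clear Enemy.
; Older sensing logic, including the SenseActor call, is left disconnected.
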(event `self.ReceiveBeginPlay`
  (`KismetSystemLibrary.PrintString` "AI System Started.")
  (bind _blackboardcomponent (`self.UseBlackboard` "/Game/Dynamic/NPC/AI/PatrolData.PatrolData"))
  (`self.RunBehaviorTree` "/Game/Dynamic/NPC/AI/GuardBehavior.GuardBehavior")
  (bind _output_get (set `self.BlackboardComp` _blackboardcomponent))
  (`BlackboardComponent.SetValueAsBool` _output_get (`self.True`) true))

(event `self.ReceiveTick`
  (params (DeltaSeconds :type "Float (single-precision)")))

(event `self.AIPerception.OnTargetPerceptionUpdated`
  (params (Actor :type "Actor Object Reference") (Stimulus :type "AIStimulus Structure"))
  (bind _blackboardcomp (`self.BlackboardComp`))
  (bind _enemy (`self.Enemy`))
  (bind _seesplayer (`self.SeesPlayer`))
  (bind _blackboardcomp_2 (`self.BlackboardComp`))
  (bind _hearsplayer (`self.HearsPlayer`))
  (bind (_age _expirationage _strength _stimuluslocation _receiverlocation _tag _bsuccessfullysensed) (break `AIStimulus` (`self.Stimulus`)))
  (if (not (`self.ActorHasTag` Actor "Enemy"))
    (bind _output_get (set `self.SensedActor` Actor))
    (bind _info (`AIPerceptionComponent.GetActorsPerception` (`self.AIPerception`) _output_get))
    (for _array_element (`.LastSensedStimuli` (break `ActorPerceptionBlueprintInfo` _info))
      (bind _output_get_2 (set `self.Stimulus` _array_element))
      (bind _returnvalue (`AIPerceptionSystem.GetSenseClassForStimulus` _output_get_2))
      (if (== _returnvalue "/Script/AIModule.AISense_Sight")
        ;[1 1 1] Sees player?
        (if _bsuccessfullysensed
          (set `self.StimulusLocation` _stimuluslocation)
          (`BlackboardComponent.SetValueAsBool` _blackboardcomp_2 _seesplayer true)
          (`KismetSystemLibrary.PrintString` "I see you!")
          (`BlackboardComponent.SetValueAsVector` _blackboardcomp (`self.LastKnownLocation`) (`self.StimulusLocation`) :!label _label)
          (`BlackboardComponent.SetValueAsObject` _blackboardcomp _enemy (`self.SensedActor`))
          (else
            (`BlackboardComponent.SetValueAsBool` _blackboardcomp_2 _seesplayer false)
            (`BlackboardComponent.ClearValue` _blackboardcomp _enemy :!label _label_2)))
        (elif (== _returnvalue "/Script/AIModule.AISense_Hearing")
          ;[1 1 1] Hears player?
          (if _bsuccessfullysensed
            (set `self.StimulusLocation` _stimuluslocation)
            (`BlackboardComponent.SetValueAsBool` _blackboardcomp_2 _hearsplayer true)
            (`KismetSystemLibrary.PrintString` "I hear you!")
            (goto _label)
            (else
              (`BlackboardComponent.SetValueAsBool` _blackboardcomp_2 _hearsplayer false)
              (goto _label_2))))))))

(fn `SenseActor`
  (params (StimulusLocation :type "Vector Structure (by ref)") (BlackboardComp :type "BlackboardComponent Object Reference (by ref)") (Enemy :type "Name (by ref)") (SensedActor :type "Actor Object Reference (by ref)"))
  (`BlackboardComponent.SetValueAsVector` BlackboardComp Enemy StimulusLocation)
  (`BlackboardComponent.SetValueAsObject` BlackboardComp Enemy SensedActor))

(fn `UserConstructionScript`)